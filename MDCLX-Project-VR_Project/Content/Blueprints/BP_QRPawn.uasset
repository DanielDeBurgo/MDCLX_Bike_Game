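; Startup pawn that pairs the game with a remote device through a QR web widget, then hands the player to the bike pawn in VR.
; It registers over Socket.IO and passes the returned URL to the widget.
; On device connection it requests the bike config and switches possession once the headset is worn, polling on Tick if needed.
; It also relays server customization, daily challenge and leaderboard events to BP_Bike_Pawn.
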(event Custom|connectedToDevice
  (bind _returnvalue (Game|GetPlayerController 0))
  ;[1 1 1] Check whether the player has the hmd on
  (Class|SocketIOClientComponent|Emit (Variables|Default|GetsocketIOClientComponent) "getBikeConfig" 0 "/")
  (if (Utilities|Enum|Equal(Enum) (Class|HeadMountedDisplayFunctionLibrary|GetHMDWornState) "Worn")
    (Utilities|FlowControl|DoOnce false
      (:Completed
        ;[1 1 1] Possessing
        (Rendering|SetActorHiddenInGame true)
        (Class|HeadMountedDisplayFunctionLibrary|EnableHMD true)
        (Pawn|UnPossess _returnvalue)
        (Pawn|Possess _returnvalue (Variables|Default|GetbikePawn))
        (Audio|PlaySound2D "/Game/Sounds/background_Cue.background_Cue" 1.0 1.0 0.0 0 0)))
    (else
      (Variables|Default|SethasConnected true)
      (bind _asbp_qr_widget (Utilities|Casting|CastToBP_QR_Widget (UserInterface|GetUserWidgetObject (Variables|Default|GetwebsiteComponent))))
      (Widget|SetVisibility (Variables|/Game/QR/BP_QR_Widget.BP_QR_Widget_C|GetWebBrowser_63 _asbp_qr_widget) "Hidden")
      (Widget|SetVisibility (Variables|/Game/QR/BP_QR_Widget.BP_QR_Widget_C|GetImage_59 _asbp_qr_widget) "Visible"))))

(event Custom|bikeConfigReturn
  (params (Message :type SIO%20Json%20Value%20Object%20Reference))
  ;[1 1 1] Set the initial bike configuration
  (bind _asbp_bike_pawn (Utilities|Casting|CastToBP_Bike_Pawn (Variables|Default|GetbikePawn)))
  (Default|SetInitialBikeConfig _asbp_bike_pawn Message))

(event Custom|changeMiscColour
  (params (Message :type SIO%20Json%20Value%20Object%20Reference))
  ;[1 1 1] Changes the misc color
  (bind _asbp_bike_pawn (Utilities|Casting|CastToBP_Bike_Pawn (Variables|Default|GetbikePawn)))
  (Default|ChangeMiscColour _asbp_bike_pawn Message))

(event Custom|registerSuccess
  (params (Message :type SIO%20Json%20Value%20Object%20Reference))
  (bind _socketioclientcomponent (Variables|Default|GetsocketIOClientComponent))
  ;[1 1 1] Binding the events
  (bind _asbp_qr_widget (Utilities|Casting|CastToBP_QR_Widget (UserInterface|GetUserWidgetObject (Variables|Default|GetwebsiteComponent))))
  (Variables|/Script/BikeProject.QRWidget|Seturl _asbp_qr_widget (Class|SIOJsonValue|AsString Message))
  (Class|SocketIOClientComponent|BindEventtoFunction _socketioclientcomponent "changeBikeColour" "changeBikeColour" 0 "/")
  (Class|SocketIOClientComponent|BindEventtoFunction _socketioclientcomponent "changeSpokeColour" "changeSpokeColour" 0 "/")
  (Class|SocketIOClientComponent|BindEventtoFunction _socketioclientcomponent "changeBikeModel" "changeBikeModel" 0 "/")
  (Class|SocketIOClientComponent|BindEventtoFunction _socketioclientcomponent "changeMiscModel" "changeMiscModel" 0 "/")
  (Class|SocketIOClientComponent|BindEventtoFunction _socketioclientcomponent "changeMiscColour" "changeMiscColour" 0 "/")
  (Class|SocketIOClientComponent|BindEventtoFunction _socketioclientcomponent "changeMiscPosition" "changeMiscPosition" 0 "/")
  (Class|SocketIOClientComponent|BindEventtoFunction _socketioclientcomponent "setDailyChallenge" "setDailyChallenge" 0 "/")
  (Class|SocketIOClientComponent|BindEventtoFunction _socketioclientcomponent "serverSentCurrentLeaderboard" "serverSentCurrentLeaderboard" 0 "/"))

(event Custom|changeBikeColour
  (params (Message :type SIO%20Json%20Value%20Object%20Reference))
  ;[1 1 1] Change the bike color
  (bind _asbp_bike_pawn (Utilities|Casting|CastToBP_Bike_Pawn (Variables|Default|GetbikePawn)))
  (Default|ChangeBikeColour _asbp_bike_pawn Message))

(event Custom|setDailyChallenge
  (params (Message :type SIO%20Json%20Value%20Object%20Reference))
  ;[1 1 1] Set the daily challenge
  (bind _asbp_bike_pawn (Utilities|Casting|CastToBP_Bike_Pawn (Variables|Default|GetbikePawn)))
  (Default|SetDailyChallenge _asbp_bike_pawn Message))

(event Custom|changeSpokeColour
  (params (Message :type SIO%20Json%20Value%20Object%20Reference))
  ;[1 1 1] Change the spoke color
  (bind _asbp_bike_pawn (Utilities|Casting|CastToBP_Bike_Pawn (Variables|Default|GetbikePawn)))
  (Default|ChangeSpokeColour _asbp_bike_pawn Message))

(event Custom|serverSentCurrentLeaderboard
  (params (Message :type SIO%20Json%20Value%20Object%20Reference))
  ;[1 1 1] Receive the leaderboard
  (bind _asbp_bike_pawn (Utilities|Casting|CastToBP_Bike_Pawn (Variables|Default|GetbikePawn)))
  (Default|ServerSentCurrentLeaderboard _asbp_bike_pawn Message))

(event Custom|changeBikeModel
  (params (Message :type SIO%20Json%20Value%20Object%20Reference))
  ;[1 1 1] Change the bike model
  (bind _asbp_bike_pawn (Utilities|Casting|CastToBP_Bike_Pawn (Variables|Default|GetbikePawn)))
  (Default|ChangeBikeModel _asbp_bike_pawn Message))

(event Custom|changeMiscModel
  (params (Message :type SIO%20Json%20Value%20Object%20Reference))
  ;[1 1 1] Changes the misc model
  (bind _asbp_bike_pawn (Utilities|Casting|CastToBP_Bike_Pawn (Variables|Default|GetbikePawn)))
  (Default|ChangeMiscModel _asbp_bike_pawn Message))

(event Custom|changeMiscPosition
  (params (Message :type SIO%20Json%20Value%20Object%20Reference))
  ;[1 1 1] Changes the misc position
  (bind _asbp_bike_pawn (Utilities|Casting|CastToBP_Bike_Pawn (Variables|Default|GetbikePawn)))
  (Default|ChangeMiscPosition _asbp_bike_pawn Message))

(event EventBeginPlay
  (bind _socketioclientcomponent (Variables|Default|GetsocketIOClientComponent))
  ;[1 1 1] Begin play connect and declare functions
  (Input|EnableInput (Game|GetPlayerController 0))
  (Class|HeadMountedDisplayFunctionLibrary|EnableHMD false)
  (Utilities|FlowControl|DoOnce false
    (:Completed
      (Class|SocketIOClientComponent|Connect _socketioclientcomponent (Variables|Default|Geturl) 0 0)
      (Class|SocketIOClientComponent|Emit _socketioclientcomponent "register" (Class|SIOJsonValue|ConstructJsonValueBool true) "/")
      (Class|SocketIOClientComponent|BindEventtoFunction _socketioclientcomponent "registerSuccess" "registerSuccess" 0 "/")
      (Class|SocketIOClientComponent|BindEventtoFunction _socketioclientcomponent "connectedToDevice" "connectedToDevice" 0 "/")
      (Class|SocketIOClientComponent|BindEventtoFunction _socketioclientcomponent "bikeConfigReturn" "bikeConfigReturn" 0 "/"))))

(event EventTick
  (params (DeltaSeconds :type Float%20%28single-precision%29))
  (bind _returnvalue (Game|GetPlayerController 0))
  ;[1 1 1] Checking on tick whether the player has connected and has the worn state true
  (Utilities|FlowControl|DoOnce false :!label _label
    (:Completed
      (if (and (Variables|Default|GethasConnected) (Utilities|Enum|Equal(Enum) (Class|HeadMountedDisplayFunctionLibrary|GetHMDWornState) "Worn"))
        (Utilities|FlowControl|DoOnce false
          (:Completed
            ;[1 1 1] Possessing
            (Rendering|SetActorHiddenInGame true)
            (Class|HeadMountedDisplayFunctionLibrary|EnableHMD true)
            (Pawn|UnPossess _returnvalue)
            (Pawn|Possess _returnvalue (Variables|Default|GetbikePawn))
            (Audio|PlaySound2D "/Game/Sounds/background_Cue.background_Cue" 1.0 1.0 0.0 0 0)))
        (else
          (goto _label Reset))))))

(event Input|KeyboardEvents|X
  (params (Key :type Key%20Structure))
  (bind _returnvalue (Game|GetPlayerController 0))
  ;[1 1 1] DEBUG
  (:Pressed
    ;[1 1 1] Check whether the player has the hmd on
    (Class|SocketIOClientComponent|Emit (Variables|Default|GetsocketIOClientComponent) "getBikeConfig" 0 "/")
    (if (Utilities|Enum|Equal(Enum) (Class|HeadMountedDisplayFunctionLibrary|GetHMDWornState) "Worn")
      (Utilities|FlowControl|DoOnce false
        (:Completed
          ;[1 1 1] Possessing
          (Rendering|SetActorHiddenInGame true)
          (Class|HeadMountedDisplayFunctionLibrary|EnableHMD true)
          (Pawn|UnPossess _returnvalue)
          (Pawn|Possess _returnvalue (Variables|Default|GetbikePawn))
          (Audio|PlaySound2D "/Game/Sounds/background_Cue.background_Cue" 1.0 1.0 0.0 0 0)))
      (else
        (Variables|Default|SethasConnected true)
        (bind _asbp_qr_widget (Utilities|Casting|CastToBP_QR_Widget (UserInterface|GetUserWidgetObject (Variables|Default|GetwebsiteComponent))))
        (Widget|SetVisibility (Variables|/Game/QR/BP_QR_Widget.BP_QR_Widget_C|GetWebBrowser_63 _asbp_qr_widget) "Hidden")
        (Widget|SetVisibility (Variables|/Game/QR/BP_QR_Widget.BP_QR_Widget_C|GetImage_59 _asbp_qr_widget) "Visible")))))

(fn ConstructionScript)