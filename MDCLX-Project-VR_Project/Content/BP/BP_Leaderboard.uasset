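; Leaderboard display that writes a passed-in leaderboard string to a TextRender under a "Leaderboard:" heading.
; It starts hidden, appears when displayLeaderboard or leaderboardTimer fires, and the latter starts a timer that hides it again.
; ParseLeaderboardString is unused by the event graph and only prints the first line's comma-separated fields.
; Its column-formatting code, which calls AddSpacesBeforeAfter, is disconnected.
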(event Custom|displayLeaderboard
  (params (Leaderboard :type SIO%20Json%20Value%20Object%20Reference))
  ;[1 1 1] Leaderboard
  (Rendering|SetVisibility (Variables|Default|GetDefaultSceneRoot) true true)
  (CallFunction|ClearLeaderboard)
  (Variables|Default|SetLeaderboardStringValue (Utilities|String|Append (Variables|Default|GetLeaderboardStringValue) " 
" (Class|SIOJsonValue|AsString Leaderboard)))
  (Rendering|Components|TextRender|SetText (Variables|Default|GetTextRender) (Utilities|Text|ToText(String) (Variables|Default|GetLeaderboardStringValue))))

(event Custom|leaderboardCloseUp
  ;[1 1 1] Timer Finish
  (Utilities|Time|ClearandInvalidateTimerbyHandle (Variables|Default|GetTimerHandle))
  (Rendering|SetVisibility (Variables|Default|GetDefaultSceneRoot) false true))

(event Custom|leaderboardTimer
  ;[1 1 1] Timer Start
  (Rendering|SetVisibility (Variables|Default|GetDefaultSceneRoot) true true)
  (bind _returnvalue (Utilities|Time|SetTimerbyFunctionName 0 "leaderboardCloseUp" 3e+01))
  (Variables|Default|SetTimerHandle _returnvalue))

(event Custom|clearLeaderboard
  ;[1 1 1] Clears the leaderboard
  (Variables|Default|SetLeaderboardStringValue "Leaderboard: 
")
  (Rendering|Components|TextRender|SetText (Variables|Default|GetTextRender) (Utilities|Text|ToText(String) (Variables|Default|GetLeaderboardStringValue))))

(event EventBeginPlay
  ;[1 1 1] Set visibility on begin
  (Rendering|SetVisibility (Variables|Default|GetDefaultSceneRoot) false true))

(fn ConstructionScript)

(fn ParseLeaderboardString
  (params (InputString :type String))
  (bind _output_get (LocalVariables|SetLeaderboardEntries (Utilities|String|ParseIntoArray InputString "LINE_TERMINATOR")))
  (bind _array_element (Utilities|Array|ForEachLoopwithBreak _output_get :!label _label)
    (:LoopBody
      (for _array_element_2 (Utilities|String|ParseIntoArray _array_element "," false)
        (Development|PrintString _array_element_2 true true "(R=0.000000,G=0.660000,B=1.000000,A=1.000000)" 1e+01))
      (goto _label Break))))

(fn AddSpacesBeforeAfter
  (params (Token :type String) (Position :type Integer%20%28by%20ref%29))
  (bind _positionchars (LocalVariables|GetPositionChars))
  (bind _output (Utilities|Array|Get(acopy) _positionchars Position))
  (bind _output_get (LocalVariables|SetSize (Utilities|String|Len Token)))
  (if (> _output_get _output)
    (LocalVariables|SetCopyOfToken (Utilities|String|GetSubstring Token 0 _output))
    (else
      (LocalVariables|SetCopyOfToken Token)))
  (if (== (Math|Integer|%(Integer) (- _output _output_get) 2) 0)
    (for _index (range 0 (/ (LocalVariables|GetSize) 2)) :!label _label
      (LocalVariables|SetCopyOfToken (Utilities|String|Append " " (LocalVariables|GetCopyOfToken))))
    (for _index_2 (range (/ (LocalVariables|GetSize) 2) (LocalVariables|GetSize))
      (LocalVariables|SetCopyOfToken (Utilities|String|Append (LocalVariables|GetCopyOfToken) " ")))
    (else
      (LocalVariables|SetCopyOfToken (Utilities|String|Append (LocalVariables|GetCopyOfToken) " "))
      (Math|Integer|DecrementInt (LocalVariables|GetSize)
        (:%20%20
          (if (> (LocalVariables|GetSize) 0)
            (goto _label)
            (else
              _))))))
  (return (LocalVariables|GetCopyOfToken)))