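; BP_Gate is a trigger gate that starts either an Uber Eats or a Checkpoints event when the bike pawn rides through it.
; GateType sets the text label, both in the construction script and at runtime through changeEvent.
; On first overlap it starts the matching timer on BP_Bike_Pawn, also spawning checkpoints from every BP_SpawningPoints in Checkpoints mode.
; It then plays a collect sound and destroys itself.
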(event OnComponentBeginOverlap(ColliderBox)
  (params (OverlappedComponent :type Primitive%20Component%20Object%20Reference) (OtherActor :type Actor%20Object%20Reference) (OtherComp :type Primitive%20Component%20Object%20Reference) (OtherBodyIndex :type Integer) (bFromSweep :type Boolean) (SweepResult :type Hit%20Result%20Structure%20%28by%20ref%29))
  (if (== (Utilities|GetClass OtherActor) "/Game/Bike/BP_Bike_Pawn.BP_Bike_Pawn_C")
    (Utilities|FlowControl|DoOnce false
      (:Completed
        (bind _asbp_bike_pawn (Utilities|Casting|CastToBP_Bike_Pawn OtherActor))
        (Utilities|FlowControl|Sequence
          (:then_0
            (switch Utilities|FlowControl|Switch|SwitchonGateType (Variables|Default|GetGateType)
              (:NewEnumerator1
                (Default|TimerUberEats _asbp_bike_pawn))
              (:NewEnumerator2
                (bind _outactors (Actor|GetAllActorsOfClass "/Game/BP/BP_SpawningPoints.BP_SpawningPoints_C"))
                (for _array_element _outactors
                  (Default|SpawnCheckpoints _array_element))
                (Default|TimerCheckpoint _asbp_bike_pawn))))
          (:then_1
            (Audio|PlaySound2D "/Game/Sounds/checkpointCollect_Cue.checkpointCollect_Cue" 1.0 1.0 0.0 0 0))
          (:then_2
            (Actor|DestroyActor)))))))

(event Custom|changeEvent
  (params (Type :type GateType%20Enum :default "NewEnumerator1"))
  (bind _text (Variables|Default|GetText))
  ;[1 1 1] Change game event
  (Variables|Default|SetGateType Type)
  (switch Utilities|FlowControl|Switch|SwitchonGateType (Variables|Default|GetGateType)
    (:NewEnumerator1
      (Rendering|Components|TextRender|SetText _text (Utilities|Text|MakeLiteralText "Uber Eats")))
    (:NewEnumerator2
      (Rendering|Components|TextRender|SetText _text (Utilities|Text|MakeLiteralText "Checkpoints")))))

(fn ConstructionScript
  (bind _text (Variables|Default|GetText))
  (switch Utilities|FlowControl|Switch|SwitchonGateType (Variables|Default|GetGateType)
    (:NewEnumerator1
      (Rendering|Components|TextRender|SetText _text (Utilities|Text|MakeLiteralText "Uber Eats")))
    (:NewEnumerator2
      (Rendering|Components|TextRender|SetText _text (Utilities|Text|MakeLiteralText "Checkpoints")))))