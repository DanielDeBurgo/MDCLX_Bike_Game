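; BP_SpawningPoints is an actor that scatters a configurable number of BP_Checkpoint actors at random positions within an area.
; Its SpawnCheckpoints event reads the world locations of the first two points of its Spline as opposite corners of a horizontal rectangle.
; It then spawns NumberOfSpawnTargets checkpoints at random X/Y positions inside those bounds, all at a fixed world height.
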(event Custom|SpawnCheckpoints
  (bind _spline (Variables|Default|GetSpline))
  (bind _returnvalue (Spline|GetLocationatSplinePoint _spline 0 "World"))
  (bind _returnvalue_2 (Spline|GetLocationatSplinePoint _spline 1 "World"))
  (bind (_x _y) (Math|Vector|BreakVector _returnvalue))
  (bind (_x_2 _y_2) (Math|Vector|BreakVector _returnvalue_2))
  (Variables|Default|SetBottomX _x)
  (Variables|Default|SetTopX _x_2)
  (Variables|Default|SetBottomY _y)
  (Variables|Default|SetTopY _y_2)
  (for _index (range 1 (Variables|Default|GetNumberOfSpawnTargets))
    (Game|SpawnActorfromClass "/Game/BP/BP_Checkpoint.BP_Checkpoint_C" (Math|Transform|MakeTransform (Math|Vector|MakeVector (Math|Random|RandomFloatinRange (Variables|Default|GetBottomX) (Variables|Default|GetTopX)) (Math|Random|RandomFloatinRange (Variables|Default|GetBottomY) (Variables|Default|GetTopY)) 1.5e+02)) "Undefined" 0 0)))

(fn ConstructionScript)