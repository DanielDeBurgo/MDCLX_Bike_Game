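; Delivery checkpoint for the bike game, acting as either a pickup (Source) or drop-off (Target) by Type.
; Overlapping a source hides all sources, reveals a random target and starts a timer scaled by distance.
; Tick displays the countdown and turns the pawn's GPS arrow toward the target.
; Reaching the target updates score and clears the source's timer via the pawn's reference, while expiry fails the delivery; both restore the sources.
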(event OnComponentBeginOverlap(Box)
  (params (OverlappedComponent :type Primitive%20Component%20Object%20Reference) (OtherActor :type Actor%20Object%20Reference) (OtherComp :type Primitive%20Component%20Object%20Reference) (OtherBodyIndex :type Integer) (bFromSweep :type Boolean) (SweepResult :type Hit%20Result%20Structure%20%28by%20ref%29))
  (bind _bikepawnref (Variables|Default|GetBikePawnRef))
  (bind _arrowgps (Variables|/Game/Bike/BP_Bike_Pawn.BP_Bike_Pawn_C|GetArrowGPS _bikepawnref))
  ;[1 1 1] Get new delivery
  (bind _asbp_bike_pawn (Utilities|Casting|CastToBP_Bike_Pawn OtherActor))
  (Utilities|FlowControl|DoOnce false :!label _label
    (:Completed
      (switch Utilities|FlowControl|Switch|SwitchonUberTargetType (Variables|Default|GetType)
        (:NewEnumerator1
          (Audio|PlaySound2D "/Game/Sounds/orderCollect_Cue.orderCollect_Cue" 1.0 1.0 0.0 0 0)
          (Variables|/Game/Bike/BP_Bike_Pawn.BP_Bike_Pawn_C|SetUberSourceRef (Variables|Default|GetBikePawnRef) self)
          (for _array_element (Variables|/Game/Bike/BP_Bike_Pawn.BP_Bike_Pawn_C|GetUberSources _asbp_bike_pawn)
            (CallFunction|Hide _array_element))
          (bind _output_get (Variables|Default|SetUberTargetRef (Utilities|Array|Get(acopy) (Variables|/Game/Bike/BP_Bike_Pawn.BP_Bike_Pawn_C|GetUberTargets _asbp_bike_pawn) (Math|Random|RandomIntegerinRange 0 (- (Utilities|Array|Length (Variables|/Game/Bike/BP_Bike_Pawn.BP_Bike_Pawn_C|GetUberTargets _asbp_bike_pawn)) 1)))))
          (CallFunction|Show _output_get)
          (CallFunction|StartTimer)
          (Development|SetHiddeninGame _arrowgps false false)
          (goto _label Reset))
        (:NewEnumerator2
          (Audio|PlaySound2D "/Game/Sounds/checkpointCollect_Cue.checkpointCollect_Cue" 1.0 1.0 0.0 0 0)
          (for _array_element_2 (Variables|/Game/Bike/BP_Bike_Pawn.BP_Bike_Pawn_C|GetUberSources _asbp_bike_pawn)
            (CallFunction|Show _array_element_2))
          (CallFunction|Hide)
          (CallFunction|WinTarget)
          (Development|SetHiddeninGame _arrowgps true false)
          (goto _label Reset))))))

(event Custom|StartTimer
  ;[1 1 1] Start Timer
  (bind _returnvalue (Utilities|Time|SetTimerbyFunctionName 0 "LostTarget" (/ (Transformation|GetDistanceTo (Variables|Default|GetUberTargetRef)) (Variables|Default|GetmaxDist))))
  (Variables|Default|SetTimerHandle _returnvalue))

(event Custom|LostTarget
  (bind _bikepawnref (Variables|Default|GetBikePawnRef))
  (bind _bikepawnref_2 (Variables|Default|GetBikePawnRef))
  (bind _arrowgps (Variables|/Game/Bike/BP_Bike_Pawn.BP_Bike_Pawn_C|GetArrowGPS _bikepawnref))
  ;[1 1 1] Lost Target
  (Audio|PlaySound2D "/Game/Sounds/orderFail_Cue.orderFail_Cue" 1.0 1.0 0.0 0 0)
  (Utilities|Time|ClearandInvalidateTimerbyHandle (Variables|Default|GetTimerHandle))
  (Rendering|Components|TextRender|SetText (Variables|/Game/Bike/BP_Bike_Pawn.BP_Bike_Pawn_C|GetCongratsText (Variables|Default|GetBikePawnRef)) (Utilities|Text|ToText(String) (Utilities|String|Append "Delivery lost. Look for next delivery" "!!")))
  (for _array_element (Variables|/Game/Bike/BP_Bike_Pawn.BP_Bike_Pawn_C|GetUberSources _bikepawnref_2)
    (CallFunction|Show _array_element))
  (CallFunction|Hide (Variables|Default|GetUberTargetRef))
  (Variables|Default|SetUberTargetRef 0)
  (Development|SetHiddeninGame (Variables|/Game/Bike/BP_Bike_Pawn.BP_Bike_Pawn_C|GetArrowGPS _bikepawnref_2) true false)
  ;[1 1 1] Get new delivery
  (Utilities|FlowControl|DoOnce false) ; enters at Reset
)

(event Custom|WinTarget
  (bind _bikepawnref (Variables|Default|GetBikePawnRef))
  ;[1 1 1] Calculate score
  (Variables|/Game/Bike/BP_Bike_Pawn.BP_Bike_Pawn_C|SetScore _bikepawnref (Math|Float|Truncate (+ (* (Utilities|Time|GetTimerRemainingTimebyHandle (Variables|Default|GetTimerHandle)) (Math|Trig|GetPI)) (Math|Conversions|ToFloat(Integer) (Variables|/Game/Bike/BP_Bike_Pawn.BP_Bike_Pawn_C|GetScore _bikepawnref)))))
  (Utilities|Time|ClearandInvalidateTimerbyHandle (Variables|BP_UberPoint_C|GetTimerHandle (Variables|/Game/Bike/BP_Bike_Pawn.BP_Bike_Pawn_C|GetUberSourceRef (Variables|Default|GetBikePawnRef))))
  (Rendering|Components|TextRender|SetText (Variables|/Game/Bike/BP_Bike_Pawn.BP_Bike_Pawn_C|GetCongratsText _bikepawnref) (Utilities|Text|ToText(String) (Utilities|String|Append "Look for next delivery" "!!"))))

(event Custom|ArrowRotation
  (bind _bikepawnref (Variables|Default|GetBikePawnRef))
  (bind _arrowgps (Variables|/Game/Bike/BP_Bike_Pawn.BP_Bike_Pawn_C|GetArrowGPS _bikepawnref))
  ;[1 1 1] Get new delivery
  (Transformation|SetWorldRotation _arrowgps (Math|Rotator|FindLookatRotation (Transformation|GetWorldLocation _arrowgps) (Transformation|GetWorldLocation (Variables|BP_UberPoint_C|GetCube (stale OnComponentBeginOverlap(Box) _output_get)))) false false))

(event EventTick
  (params (DeltaSeconds :type Float%20%28single-precision%29))
  (bind _timerhandle (Variables|Default|GetTimerHandle))
  (bind _bikepawnref (Variables|Default|GetBikePawnRef))
  (bind _timerhandle_2 (Variables|Default|GetTimerHandle))
  (bind _returnvalue (Utilities|Time|GetTimerRemainingTimebyHandle _timerhandle_2))
  (bind _congratstext (Variables|/Game/Bike/BP_Bike_Pawn.BP_Bike_Pawn_C|GetCongratsText _bikepawnref))
  (bind _returnvalue_2 (/ _returnvalue 6e+01))
  (bind _returnvalue_3 (Math|Float|%(Float) _returnvalue 6e+01))
  (bind _returnvalue_4 (Math|Float|Floor _returnvalue_2))
  (bind _returnvalue_5 (Math|Float|Floor _returnvalue_3))
  (bind _returnvalue_6 (Utilities|String|ToString(Integer) _returnvalue_4))
  (bind _returnvalue_7 (Utilities|String|ToString(Integer) _returnvalue_5))
  ;[1 1 1] Tick timer
  (if (and (Utilities|Time|IsTimerActivebyHandle _timerhandle) (Class|KismetSystemLibrary|TimerExistsHandle _timerhandle))
    (Utilities|FlowControl|Sequence
      (:then_0
        (if (< _returnvalue_5 10)
          (Rendering|Components|TextRender|SetText _congratstext (Utilities|Text|ToText(String) (Utilities|String|Append "Delivery time: " _returnvalue_6 ":" "0" _returnvalue_7)))
          (else
            (Rendering|Components|TextRender|SetText _congratstext (Utilities|Text|ToText(String) (Utilities|String|Append "Delivery time: " _returnvalue_6 ":" _returnvalue_7))))))
      (:then_1
        (if (!= (Variables|Default|GetUberTargetRef) 0)
          (CallFunction|ArrowRotation))))
    (else
      (Rendering|Components|TextRender|SetText _congratstext (Variables|Default|GetDefaultStringTime)))))

(event EventBeginPlay
  ;[1 1 1] Hide the uber points
  (bind _outactors (Actor|GetAllActorsOfClass "/Game/Bike/BP_Bike_Pawn.BP_Bike_Pawn_C"))
  (Variables|Default|SetBikePawnRef (Utilities|Array|Get(acopy) _outactors))
  (CallFunction|Hide))

(fn ConstructionScript
  (bind _cube (Variables|Default|GetCube))
  (switch Utilities|FlowControl|Switch|SwitchonUberTargetType (Variables|Default|GetType)
    (:NewEnumerator1
      (Rendering|Material|SetMaterial _cube 0 "/Game/Models/Materials/MI_Checkpoint_From.MI_Checkpoint_From"))
    (:NewEnumerator2
      (Rendering|Material|SetMaterial _cube 0 "/Game/Models/Materials/MI_Checkpoint_To.MI_Checkpoint_To"))))

(fn Hide
  (Collision|SetCollisionEnabled (Variables|Default|GetBox) "NoCollision")
  (Rendering|SetActorHiddenInGame true))

(fn Show
  (Collision|SetCollisionEnabled (Variables|Default|GetBox) "QueryAndPhysics")
  (Rendering|SetActorHiddenInGame false))