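; VR bike pawn with timed checkpoint and Uber Eats challenges that award bike-hire credits.
; Right-controller yaw steers the handlebar and the frame interpolates after it; thumbstick presses accelerate, triggers brake, arrow keys offer keyboard control.
; Message-driven events set the daily challenge and customise meshes, accessories and colours through dynamic materials.
; Challenge ends send results over Socket.IO and request the leaderboard, shown on a child actor.
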(event Custom|RotateBikeBack
  ;[1 1 1] Back rot
  (Transformation|SetWorldRotation (Variables|Default|GetBikeMiddle) (Math|Rotator|MakeRotator 0.0 0.0 (.Yaw (Math|Rotator|BreakRotator (Math|Interpolation|RInterpTo (Transformation|GetWorldRotation (Variables|Default|GetBikeMiddle)) (Transformation|GetWorldRotation (Variables|Default|GetHandle)) (stale EventTick DeltaSeconds) (* (Variables|Default|GetInterpSpeed) (* (Variables|Default|Getacceleration) (Variables|Default|Getspeed))))))) false false))

(event Custom|CheckpointMode
  ;[1 1 1] End global checkpoint timer
  (Class|SocketIOClientComponent|Emit (Variables|Default|GetsocketIOClientComponent) "sendResults" (Class|SIOJsonValue|ConstructJsonValueArray (Utilities|Array|MakeArray (Class|SIOJLibrary|ToJsonValue(Float) (Class|KismetSystemLibrary|GetTimerElapsedTimeHandle (Variables|Default|GetTimerHandle))) (Class|SIOJLibrary|ToJsonValue(Float) (Math|Float|Clamp(Float) (Math|Conversions|ToFloat(Integer) (Variables|Default|GetScore)) 0.0 5e+02)))) "/")
  (Utilities|Time|ClearandInvalidateTimerbyHandle (Variables|Default|GetTimerHandle))
  (Rendering|Components|TextRender|SetText (Variables|Default|GetTimerText) (Utilities|Text|ToText(String) (Utilities|String|Append "Time's up! " "You have received " (Utilities|String|ToString(Integer) (Variables|Default|GetScore)) " credits for bike hiring!")))
  (CallFunction|ServerSendCurrentLeaderboard)
  (Audio|PlaySound2D "/Game/Sounds/win_Cue.win_Cue" 1.0 1.0 0.0 0 0)
  (bind _outactors (Actor|GetAllActorsOfClass "/Game/BP/BP_Checkpoint.BP_Checkpoint_C"))
  (for _array_element _outactors
    (Actor|DestroyActor _array_element)))

(event Custom|changeMiscColour
  (params (Message :type SIO%20Json%20Value%20Object%20Reference))
  (bind _returnvalue (Class|SIOJsonValue|AsString Message))
  (bind (_outconvertedcolor _outisvalid) (Math|Conversions|ToColor(LinearColor) _returnvalue))
  ;[1 1 1] Misc Color
  (if _outisvalid
    (for _array_element (Variables|Default|GetMiscColorDynamicMats)
      (Rendering|Material|SetVectorParameterValue _array_element "Color" _outconvertedcolor :!class /Script/Engine.MaterialInstanceDynamic))))

(event Custom|CreateDynamicMats
  (bind _bikecolordynamicmats (Variables|Default|GetBikeColorDynamicMats))
  (bind _spokecolordynamicmats (Variables|Default|GetSpokeColorDynamicMats))
  (bind _frontmisc (Variables|Default|GetFrontMisc))
  (bind _misccolordynamicmats (Variables|Default|GetMiscColorDynamicMats))
  (bind _backmisc (Variables|Default|GetBackMisc))
  (bind _bikecolordynamicmats_2 (Variables|Default|GetBikeColorDynamicMats))
  ;[1 1 1] Initialize the arrays of dynamic materials
  (Utilities|FlowControl|Sequence
    (:then_0
      (bind _returnvalue (Rendering|Material|CreateDynamicMaterialInstance _frontmisc 1 "/Game/Models/Materials/MI_PlasticMisc.MI_PlasticMisc" "None" :!class /Script/Engine.PrimitiveComponent))
      (Utilities|Array|AddUnique _misccolordynamicmats _returnvalue))
    (:then_1
      (bind _returnvalue_2 (Rendering|Material|CreateDynamicMaterialInstance _backmisc 0 "/Game/Models/Materials/MI_PlasticMisc.MI_PlasticMisc" "None" :!class /Script/Engine.PrimitiveComponent))
      (Utilities|Array|AddUnique _misccolordynamicmats _returnvalue_2))
    (:then_2
      (bind _returnvalue_3 (Rendering|Material|CreateDynamicMaterialInstance _frontmisc 0 "/Game/Models/Materials/MI_BikeColor.MI_BikeColor" "None" :!class /Script/Engine.PrimitiveComponent))
      (Utilities|Array|AddUnique _bikecolordynamicmats _returnvalue_3))
    (:then_3
      (bind _returnvalue_4 (Rendering|Material|CreateDynamicMaterialInstance _backmisc 1 "/Game/Models/Materials/MI_BikeColor.MI_BikeColor" "None" :!class /Script/Engine.PrimitiveComponent))
      (Utilities|Array|AddUnique _bikecolordynamicmats _returnvalue_4))
    (:then_4
      (bind _returnvalue_5 (Rendering|Material|CreateDynamicMaterialInstance (Variables|Default|GetBikeMiddle) 0 "/Game/Models/Materials/MI_BikeColor.MI_BikeColor" "None" :!class /Script/Engine.PrimitiveComponent))
      (Utilities|Array|AddUnique _bikecolordynamicmats_2 _returnvalue_5))
    (:then_5
      (bind _returnvalue_6 (Rendering|Material|CreateDynamicMaterialInstance (Variables|Default|GetHandle) 1 "/Game/Models/Materials/MI_BikeColor.MI_BikeColor" "None" :!class /Script/Engine.PrimitiveComponent))
      (Utilities|Array|AddUnique _bikecolordynamicmats_2 _returnvalue_6))
    (:then_6
      (bind _returnvalue_7 (Rendering|Material|CreateDynamicMaterialInstance (Variables|Default|GetBackSpoke) 0 "/Game/Models/Materials/MI_BikeSpoke.MI_BikeSpoke" "None" :!class /Script/Engine.PrimitiveComponent))
      (Utilities|Array|AddUnique _spokecolordynamicmats _returnvalue_7))
    (:then_7
      (bind _returnvalue_8 (Rendering|Material|CreateDynamicMaterialInstance (Variables|Default|GetFrontSpoke) 0 "/Game/Models/Materials/MI_BikeSpoke.MI_BikeSpoke" "None" :!class /Script/Engine.PrimitiveComponent))
      (Utilities|Array|AddUnique _spokecolordynamicmats _returnvalue_8))))

(event Custom|changeMiscPosition
  (params (Message :type SIO%20Json%20Value%20Object%20Reference))
  ;[1 1 1] Change misc position
  (switch string (Class|SIOJsonValue|AsString Message)
    (:front
      (Variables|Default|SetisFront true))
    (:back
      (Variables|Default|SetisFront false)))
  (CallFunction|ChangeMiscModel (Class|SIOJLibrary|ToJsonValue(Integer) (Variables|Default|GetmiscModel))))

(event Custom|setDailyChallenge
  (params (Message :type SIO%20Json%20Value%20Object%20Reference))
  ;[1 1 1] Set Challenge
  (switch string (Class|SIOJsonValue|AsString Message)
    (:uber-eats
      (bind _output_get (Variables|Default|SetChallengeType "NewEnumerator1"))
      (bind _outactors (Actor|GetAllActorsOfClass "/Game/BP/BP_Gate.BP_Gate_C"))
      (Default|ChangeEvent (Utilities|Array|Get(acopy) _outactors) _output_get))
    (:checkpoints
      (bind _output_get_2 (Variables|Default|SetChallengeType "NewEnumerator2"))
      (bind _outactors_2 (Actor|GetAllActorsOfClass "/Game/BP/BP_Gate.BP_Gate_C"))
      (Default|ChangeEvent (Utilities|Array|Get(acopy) _outactors_2) _output_get_2))))

(event Custom|serverSentCurrentLeaderboard
  (params (Message :type SIO%20Json%20Value%20Object%20Reference))
  ;[1 1 1] Get the leaderboard from the server
  (Development|PrintString (Class|SIOJsonValue|AsString Message))
  (bind _asbp_leaderboard (Utilities|Casting|CastToBP_Leaderboard (Variables|/Script/Engine.ChildActorComponent|GetChildActor (Variables|Default|GetLeaderboard))))
  (Default|DisplayLeaderboard _asbp_leaderboard Message))

(event Custom|Decelerate
  (params (Deceleration :type Float%20%28single-precision%29))
  ;[1 1 1] Decelerate
  (if (> (Variables|Default|Getacceleration) Deceleration)
    (Variables|Default|Setacceleration (- (Variables|Default|Getacceleration) Deceleration))))

(event Custom|serverSendCurrentLeaderboard
  ;[1 1 1] Ask the server to send the leaderboard
  (Class|SocketIOClientComponent|Emit (Variables|Default|GetsocketIOClientComponent) "serverSendCurrentLeaderboard" 0 "/"))

(event Custom|SetInitialBikeConfig
  (params (Message :type SIO%20Json%20Value%20Object%20Reference))
  (bind _returnvalue (Class|SIOJsonValue|AsArray Message))
  ;[1 1 1] Set initial state
  (CallFunction|ChangeBikeColour (Utilities|Array|Get(acopy) _returnvalue))
  (CallFunction|ChangeSpokeColour (Utilities|Array|Get(acopy) _returnvalue 1))
  (CallFunction|ChangeBikeModel (Utilities|Array|Get(acopy) _returnvalue 2))
  (CallFunction|ChangeMiscModel (Utilities|Array|Get(acopy) _returnvalue 3))
  (CallFunction|ChangeMiscColour (Utilities|Array|Get(acopy) _returnvalue 4))
  (CallFunction|ChangeMiscPosition (Utilities|Array|Get(acopy) _returnvalue 5)))

(event Custom|changeBikeColour
  (params (Message :type SIO%20Json%20Value%20Object%20Reference))
  (bind _returnvalue (Class|SIOJsonValue|AsString Message))
  (bind (_outconvertedcolor _outisvalid) (Math|Conversions|ToColor(LinearColor) _returnvalue))
  ;[1 1 1] Bike Color
  (if _outisvalid
    (for _array_element (Variables|Default|GetBikeColorDynamicMats)
      (Rendering|Material|SetVectorParameterValue _array_element "Color" _outconvertedcolor :!class /Script/Engine.MaterialInstanceDynamic))))

(event Custom|UberEatsMode
  ;[1 1 1] End global ubereats timer
  (Class|SocketIOClientComponent|Emit (Variables|Default|GetsocketIOClientComponent) "sendResults" (Class|SIOJsonValue|ConstructJsonValueArray (Utilities|Array|MakeArray (Class|SIOJLibrary|ToJsonValue(Float) (Class|KismetSystemLibrary|GetTimerElapsedTimeHandle (Variables|Default|GetTimerHandle))) (Class|SIOJLibrary|ToJsonValue(Float) (Math|Float|Clamp(Float) (Math|Conversions|ToFloat(Integer) (Variables|Default|GetScore)) 0.0 5e+02)))) "/")
  (Utilities|Time|ClearandInvalidateTimerbyHandle (Variables|Default|GetTimerHandle))
  (Rendering|Components|TextRender|SetText (Variables|Default|GetTimerText) (Utilities|Text|ToText(String) (Utilities|String|Append "Time's up! " "You have received " (Utilities|String|ToString(Integer) (Variables|Default|GetScore)) " credits for bike hiring!")))
  (CallFunction|ServerSendCurrentLeaderboard)
  (Audio|PlaySound2D "/Game/Sounds/win_Cue.win_Cue" 1.0 1.0 0.0 0 0)
  (bind _outactors (Actor|GetAllActorsOfClass "/Game/BP/BP_UberPoint.BP_UberPoint_C"))
  (for _array_element _outactors
    (Utilities|Time|ClearandInvalidateTimerbyHandle (Variables|/Game/BP/BP_UberPoint.BP_UberPoint_C|GetTimerHandle _array_element))
    (Default|Hide _array_element)))

(event Custom|changeSpokeColour
  (params (Message :type SIO%20Json%20Value%20Object%20Reference))
  (bind _returnvalue (Class|SIOJsonValue|AsString Message))
  (bind (_outconvertedcolor _outisvalid) (Math|Conversions|ToColor(LinearColor) _returnvalue))
  ;[1 1 1] Spoke Color
  (if _outisvalid
    (for _array_element (Variables|Default|GetSpokeColorDynamicMats)
      (Rendering|Material|SetVectorParameterValue _array_element "Color" _outconvertedcolor :!class /Script/Engine.MaterialInstanceDynamic))))

(event Custom|TimerUberEats
  ;[1 1 1] Start timer ubereats challenge
  (bind _outactors (Actor|GetAllActorsOfClass "/Game/BP/BP_UberPoint.BP_UberPoint_C"))
  (for _array_element _outactors
    (switch Utilities|FlowControl|Switch|SwitchonUberTargetType (Variables|/Game/BP/BP_UberPoint.BP_UberPoint_C|GetType _array_element)
      (:NewEnumerator1
        (Utilities|Array|Add (Variables|Default|GetUberSources) _array_element)
        (Default|Show _array_element))
      (:NewEnumerator2
        (Utilities|Array|Add (Variables|Default|GetUberTargets) _array_element))))
  (bind _returnvalue (Utilities|Time|SetTimerbyFunctionName 0 "UberEatsMode" (Variables|Default|GetchallengesGlobalTimer)))
  (Variables|Default|SetTimerHandle _returnvalue))

(event Custom|changeBikeModel
  (params (Message :type SIO%20Json%20Value%20Object%20Reference))
  (bind _handle (Variables|Default|GetHandle))
  (bind _bikemiddle (Variables|Default|GetBikeMiddle))
  ;[1 1 1] Change bike model
  (switch int (Math|Float|Truncate (Class|SIOJsonValue|AsNumber Message))
    (:0
      (Components|StaticMesh|SetStaticMesh _handle "/Game/Models/Bike/Bike_02/frontwheel.frontwheel")
      (Components|StaticMesh|SetStaticMesh _bikemiddle "/Game/Models/Bike/Bike_02/backbike.backbike"))
    (:1
      (Components|StaticMesh|SetStaticMesh _handle "/Game/Models/Bike/Bike_03/frontwheel_03.frontwheel_03")
      (Components|StaticMesh|SetStaticMesh _bikemiddle "/Game/Models/Bike/Bike_02/backbike.backbike"))
    (:2
      (Components|StaticMesh|SetStaticMesh _handle "/Game/Models/Bike/Bike_02/frontwheel.frontwheel")
      (Components|StaticMesh|SetStaticMesh _bikemiddle "/Game/Models/Bike/Bike_04/backbike_03.backbike_03"))))

(event Custom|TimerCheckpoint
  ;[1 1 1] Start timer checkpoint challenge
  (bind _outactors (Actor|GetAllActorsOfClass "/Game/BP/BP_Checkpoint.BP_Checkpoint_C"))
  (Variables|Default|SetTotalScore (Utilities|Array|Length _outactors))
  (bind _returnvalue (Utilities|Time|SetTimerbyFunctionName 0 "CheckpointMode" (Variables|Default|GetchallengesGlobalTimer)))
  (Variables|Default|SetTimerHandle _returnvalue)
  (Rendering|Components|TextRender|SetTextRenderColor (Variables|Default|GetTimerText) (Math|Color|MakeColor 0 0 255 255)))

(event Custom|changeMiscModel
  (params (Message :type SIO%20Json%20Value%20Object%20Reference))
  (bind _frontmisc (Variables|Default|GetFrontMisc))
  ;[1 1 1] Change Misc Model
  (bind _output_get (Variables|Default|SetmiscModel (Math|Float|Truncate (Class|SIOJsonValue|AsNumber Message))))
  (switch int _output_get
    (:0
      (Rendering|SetVisibility (Variables|Default|GetBackMisc) false true)
      (if (Variables|Default|GetisFront)
        (Rendering|SetVisibility (Variables|Default|GetFrontMisc) true false)
        (else
          (Rendering|SetVisibility (Variables|Default|GetBackMisc) true false))))
    (:1
      (Rendering|SetVisibility _frontmisc false true)
      (if (Variables|Default|GetisFront)
        (Rendering|SetVisibility (Variables|Default|GetFrontBear) true false)
        (else
          (Rendering|SetVisibility (Variables|Default|GetBackBear) true false))))
    (:2
      (Rendering|SetVisibility _frontmisc false true)
      (if (Variables|Default|GetisFront)
        (Rendering|SetVisibility (Variables|Default|GetFrontBunny) true false)
        (else
          (Rendering|SetVisibility (Variables|Default|GetBackBunny) true false))))))

(event Custom|AddScore
  ;[1 1 1] Score
  (bind _result (Math|Integer|IncrementInt (Variables|Default|GetScore))
    (:%20%20
      (if (== _result (Variables|Default|GetTotalScore))
        (CallFunction|CheckpointMode)
        (Rendering|Components|TextRender|SetText (Variables|Default|GetCongratsText) (Utilities|Text|ToText(String) (Utilities|String|Append "Congrats" "!")))))))

(event EventBeginPlay
  (bind _defaultsceneroot (Variables|Default|GetDefaultSceneRoot))
  (bind _handle (Variables|Default|GetHandle))
  (bind _relativerotation (Variables|/Script/Engine.SceneComponent|GetRelativeRotation _defaultsceneroot))
  (bind (_roll _pitch _yaw) (Math|Rotator|BreakRotator _relativerotation))
  (Utilities|FlowControl|Sequence
    (:then_0
      (CallFunction|CreateDynamicMats))
    (:then_1
      (Transformation|SetRelativeRotation _handle (Variables|Default|GetInitWheelRotation) false false)
      (Variables|Default|SetInitWheelRotation (Variables|/Script/Engine.SceneComponent|GetRelativeRotation _handle))
      (Variables|Default|SetInitControllerRotation (Variables|/Script/Engine.SceneComponent|GetRelativeRotation (Variables|Default|GetMotionController_R)))
      (Transformation|SetRelativeRotation (Variables|Default|GetDefaultSceneRoot) (Math|Rotator|MakeRotator _roll _pitch _yaw) false false)
      ;[1 1 1] Unreal Bug - this fixes it
      (Transformation|AddRelativeRotation (Variables|Default|GetFrontWheel) "0,0.000000,1.000000" false false))))

(event EventTick
  (params (DeltaSeconds :type Float%20%28single-precision%29))
  (bind _timerhandle (Variables|Default|GetTimerHandle))
  (bind _timertext (Variables|Default|GetTimerText))
  (bind _motioncontroller_r (Variables|Default|GetMotionController_R))
  (bind _returnvalue (Utilities|Time|GetTimerRemainingTimebyHandle _timerhandle))
  (bind _returnvalue_2 (/ _returnvalue 6e+01))
  (bind _returnvalue_3 (Math|Float|%(Float) _returnvalue 6e+01))
  (bind _returnvalue_4 (Math|Float|Floor _returnvalue_2))
  (bind _returnvalue_5 (Math|Float|Floor _returnvalue_3))
  (bind _returnvalue_6 (Utilities|String|ToString(Integer) _returnvalue_4))
  (bind _returnvalue_7 (Utilities|String|ToString(Integer) _returnvalue_5))
  (if (Variables|Default|GetsetZero)
    (Utilities|FlowControl|Sequence
      (:then_0
        ;[1 1 1] Rotation Front wheel
        (Transformation|SetRelativeRotation (Variables|Default|GetHandle) (Math|Rotator|MakeRotator -1e+01 0.0 (.Yaw (Math|Rotator|BreakRotator (Math|Rotator|CombineRotators (Math|Rotator|CombineRotators (Variables|/Script/Engine.SceneComponent|GetRelativeRotation (Variables|Default|GetMotionController_R)) (Class|KismetMathLibrary|NegateRotator (Variables|Default|GetInitControllerRotation))) (Variables|Default|GetInitWheelRotation))))) false false)
        (CallFunction|RotateBikeBack))
      (:then_1
        ;[1 1 1] Acceleration
        (Transformation|AddActorLocalOffset (Math|Vector|MakeVector (.X (Math|Vector|BreakVector (* (Math|Vector|GetForwardVector (Transformation|GetWorldRotation (Variables|Default|GetHandle))) (* (Variables|Default|Getacceleration) (Variables|Default|Getspeed))))) (.Y (Math|Vector|BreakVector (* (Math|Vector|GetForwardVector (Transformation|GetWorldRotation (Variables|Default|GetHandle))) (* (Variables|Default|Getacceleration) (Variables|Default|Getspeed))))) 0.0) false false)
        (CallFunction|SetWheelsRotation (* (Variables|Default|Getacceleration) (Variables|Default|Getspeed))))
      (:then_2
        (if (Variables|Default|Getaccelerate)
          ;[1 1 1] Accelerate on touch
          (if (<= (Variables|Default|Getacceleration) 2e+02)
            (Variables|Default|Setacceleration (+ (Variables|Default|Getacceleration) 0.2)))
          (else
            (CallFunction|Decelerate 0.1))))
      (:then_3
        ;[1 1 1] Set Timer Text (on tick)
        (if (Class|KismetSystemLibrary|TimerExistsHandle (Variables|Default|GetTimerHandle))
          (if (< _returnvalue_5 10)
            (Rendering|Components|TextRender|SetText _timertext (Utilities|Text|ToText(String) (Utilities|String|Append "Time remaining: " _returnvalue_6 ":" "0" _returnvalue_7)))
            (else
              (Rendering|Components|TextRender|SetText _timertext (Utilities|Text|ToText(String) (Utilities|String|Append "Time remaining: " _returnvalue_6 ":" _returnvalue_7)))))))
      (:then_5
        (if (Variables|Default|GetrotateL)
          (Transformation|AddLocalRotation _motioncontroller_r "0,-0.500000, 0" false false)))
      (:then_6
        (if (Variables|Default|GetrotateR)
          (Transformation|AddLocalRotation _motioncontroller_r "0,0.500000, 0" false false))))))

(event Input|KeyboardEvents|MotionControllerRightTriggerAxis
  (params (AxisValue :type Float%20%28single-precision%29))
  ;[1 1 1] decelerate
  (if (Variables|Default|GetdecelerationR)
    (CallFunction|Decelerate (* (* AxisValue (Variables|Default|Getacceleration)) 0.005))))

(event Input|KeyboardEvents|MotionControllerLeftTriggerAxis
  (params (AxisValue :type Float%20%28single-precision%29))
  ;[1 1 1] decelerate
  (if (Variables|Default|GetdecelerationL)
    (CallFunction|Decelerate (* (* AxisValue (Variables|Default|Getacceleration)) 0.005))))

(event Input|KeyboardEvents|MotionControllerLeftThumbstick
  (params (Key :type Key%20Structure))
  (bind _defaultsceneroot (Variables|Default|GetDefaultSceneRoot))
  (bind _handle (Variables|Default|GetHandle))
  (bind _relativerotation (Variables|/Script/Engine.SceneComponent|GetRelativeRotation _defaultsceneroot))
  (bind (_roll _pitch _yaw) (Math|Rotator|BreakRotator _relativerotation))
  ;[1 1 1] Set initial handle bar position
  (:Pressed
    (Variables|Default|Setaccelerate true)
    (if (not (Variables|Default|GetsetZero))
      (Variables|Default|SetsetZero true)
      (Utilities|FlowControl|DoOnce false
        (:Completed
          (Transformation|SetRelativeRotation _handle (Variables|Default|GetInitWheelRotation) false false)
          (Variables|Default|SetInitWheelRotation (Variables|/Script/Engine.SceneComponent|GetRelativeRotation _handle))
          (Variables|Default|SetInitControllerRotation (Variables|/Script/Engine.SceneComponent|GetRelativeRotation (Variables|Default|GetMotionController_R)))
          (Transformation|SetRelativeRotation (Variables|Default|GetDefaultSceneRoot) (Math|Rotator|MakeRotator _roll _pitch _yaw) false false)
          ;[1 1 1] Unreal Bug - this fixes it
          (Transformation|AddRelativeRotation (Variables|Default|GetFrontWheel) "0,0.000000,1.000000" false false)))))
  (:Released
    (Variables|Default|Setaccelerate false)))

(event Input|KeyboardEvents|MotionControllerRightThumbstick
  (params (Key :type Key%20Structure))
  (bind _defaultsceneroot (Variables|Default|GetDefaultSceneRoot))
  (bind _handle (Variables|Default|GetHandle))
  (bind _relativerotation (Variables|/Script/Engine.SceneComponent|GetRelativeRotation _defaultsceneroot))
  (bind (_roll _pitch _yaw) (Math|Rotator|BreakRotator _relativerotation))
  ;[1 1 1] Set initial handle bar position
  (:Pressed
    (Variables|Default|Setaccelerate true)
    (if (not (Variables|Default|GetsetZero))
      (Variables|Default|SetsetZero true)
      (Utilities|FlowControl|DoOnce false
        (:Completed
          (Transformation|SetRelativeRotation _handle (Variables|Default|GetInitWheelRotation) false false)
          (Variables|Default|SetInitWheelRotation (Variables|/Script/Engine.SceneComponent|GetRelativeRotation _handle))
          (Variables|Default|SetInitControllerRotation (Variables|/Script/Engine.SceneComponent|GetRelativeRotation (Variables|Default|GetMotionController_R)))
          (Transformation|SetRelativeRotation (Variables|Default|GetDefaultSceneRoot) (Math|Rotator|MakeRotator _roll _pitch _yaw) false false)
          ;[1 1 1] Unreal Bug - this fixes it
          (Transformation|AddRelativeRotation (Variables|Default|GetFrontWheel) "0,0.000000,1.000000" false false)))))
  (:Released
    (Variables|Default|Setaccelerate false)))

(event Input|KeyboardEvents|MotionControllerLeftTrigger
  (params (Key :type Key%20Structure))
  ;[1 1 1] decelerate
  (:Pressed
    (Variables|Default|SetdecelerationL true))
  (:Released
    (Variables|Default|SetdecelerationL false)))

(event Input|KeyboardEvents|MotionControllerRightTrigger
  (params (Key :type Key%20Structure))
  ;[1 1 1] decelerate
  (:Pressed
    (Variables|Default|SetdecelerationR true))
  (:Released
    (Variables|Default|SetdecelerationR false)))

(event Input|KeyboardEvents|Up
  (params (Key :type Key%20Structure))
  (bind _defaultsceneroot (Variables|Default|GetDefaultSceneRoot))
  (bind _handle (Variables|Default|GetHandle))
  (bind _relativerotation (Variables|/Script/Engine.SceneComponent|GetRelativeRotation _defaultsceneroot))
  (bind (_roll _pitch _yaw) (Math|Rotator|BreakRotator _relativerotation))
  (:Pressed
    ;[1 1 1] Set initial handle bar position
    (Variables|Default|Setaccelerate true)
    (if (not (Variables|Default|GetsetZero))
      (Variables|Default|SetsetZero true)
      (Utilities|FlowControl|DoOnce false
        (:Completed
          (Transformation|SetRelativeRotation _handle (Variables|Default|GetInitWheelRotation) false false)
          (Variables|Default|SetInitWheelRotation (Variables|/Script/Engine.SceneComponent|GetRelativeRotation _handle))
          (Variables|Default|SetInitControllerRotation (Variables|/Script/Engine.SceneComponent|GetRelativeRotation (Variables|Default|GetMotionController_R)))
          (Transformation|SetRelativeRotation (Variables|Default|GetDefaultSceneRoot) (Math|Rotator|MakeRotator _roll _pitch _yaw) false false)
          ;[1 1 1] Unreal Bug - this fixes it
          (Transformation|AddRelativeRotation (Variables|Default|GetFrontWheel) "0,0.000000,1.000000" false false)))))
  (:Released
    (Variables|Default|Setaccelerate false)))

(event Input|KeyboardEvents|Left
  (params (Key :type Key%20Structure))
  (:Pressed
    (Variables|Default|SetrotateL true))
  (:Released
    (Variables|Default|SetrotateL false)))

(event Input|KeyboardEvents|Right
  (params (Key :type Key%20Structure))
  (:Pressed
    (Variables|Default|SetrotateR true))
  (:Released
    (Variables|Default|SetrotateR false)))

(fn ConstructionScript)

(fn SetWheelsRotation
  (params (Factor :type Float%20%28single-precision%29))
  (bind _returnvalue (Math|Rotator|MakeRotator Factor 0.0 0.0))
  (Transformation|AddRelativeRotation (Variables|Default|GetFrontWheel) _returnvalue false false)
  (Transformation|AddRelativeRotation (Variables|Default|GetBackWheel) _returnvalue false false))